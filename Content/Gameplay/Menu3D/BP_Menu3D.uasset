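; BP_Menu3D is a world-placed 3D menu actor that hands the player's view over to other linked menu actors.
; On BeginPlay it binds to the transition event of the Menu3D_Widget in its widget component, which passes an index into its LinkedMenus array.
; A valid index disables its own collision, enables the target's and eases the player's camera to that menu with a view target blend.
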(event Custom|TransitionTo
  (params (NewMenu :type BP%20Menu%203D%20Object%20Reference))
  (Collision|SetActorEnableCollision false)
  (Collision|SetActorEnableCollision NewMenu true)
  (Game|Player|SetViewTargetwithBlend (Game|GetPlayerController 0) NewMenu 1.5 "VTBlend_EaseInOut" 1.5 false))

(event Custom|TransitionToLinkedMenu_Event
  (params (MenuIndex :type Integer))
  (if (Utilities|Array|IsValidIndex (Variables|Default|GetLinkedMenus) MenuIndex)
    (CallFunction|Transitionto (Utilities|Array|Get(acopy) (Variables|Default|GetLinkedMenus) MenuIndex))))

(event EventBeginPlay
  (bind _asmenu_3d_widget (Utilities|Casting|CastToMenu3D_Widget (UserInterface|GetUserWidgetObject (Variables|Default|GetWidget))))
  (EventDispatchers|AssignTransitiontoLinkedMenu _asmenu_3d_widget (delegate Custom|TransitionToLinkedMenu_Event)))

(fn ConstructionScript)